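; Player projectile that destroys enemies on contact and awards score.
; While the player is alive, Tick moves it along world X at a multiple of the player's forward speed, keeping it ahead of the player.
; Sphere overlap destroys it on components tagged Break; on actors tagged Enemy, it passes an incremented score to BP_Player's ProcessScore, then destroys both actors.
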(event `self.ReceiveTick`
  (params (DeltaSeconds :type "Float (single-precision)"))
  (bind _asbp_player (cast `/Game/InfiniteMatrix/Blueprints/BP_Player` (`GameplayStatics.GetPlayerPawn` 0)))
  (if (not (`/Game/InfiniteMatrix/Blueprints/BP_Player.IsDead` _asbp_player))
    (`self.K2_AddActorWorldOffset` (`KismetMathLibrary.MakeVector` (* DeltaSeconds (* (`/Game/InfiniteMatrix/Blueprints/BP_Player.ForwardSpeed` _asbp_player) 1.5))))))

(event `self.Sphere.OnComponentBeginOverlap`
  (params (OverlappedComponent :type "PrimitiveComponent Object Reference") (OtherActor :type "Actor Object Reference") (OtherComp :type "PrimitiveComponent Object Reference") (OtherBodyIndex :type Integer) (bFromSweep :type Boolean) (SweepResult :type "HitResult Structure (by ref)"))
  (if (`ActorComponent.ComponentHasTag` OtherComp "Break")
    (`self.K2_DestroyActor`)
    (elif (`self.ActorHasTag` OtherActor "Enemy")
      (bind _asbp_player (cast `/Game/InfiniteMatrix/Blueprints/BP_Player` (`GameplayStatics.GetPlayerPawn` 0)))
      (`/Game/InfiniteMatrix/Blueprints/BP_Player.ProcessScore` _asbp_player (+ (`/Game/InfiniteMatrix/Blueprints/BP_Player.Score` _asbp_player) 1))
      (`self.K2_DestroyActor`)
      (`self.K2_DestroyActor` OtherActor))))

(fn `UserConstructionScript`)