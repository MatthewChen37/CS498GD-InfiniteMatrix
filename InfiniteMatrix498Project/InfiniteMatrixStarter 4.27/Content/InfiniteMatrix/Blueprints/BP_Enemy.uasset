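; BP_Enemy is an enemy actor that reacts to overlaps with the player or with projectiles.
; Overlapping a Player-tagged actor calls ProcessHit on that BP_Player, while overlapping a Projectile-tagged actor raises the first player pawn's score by one through ProcessScore.
; Both cases then destroy the enemy, which has no movement or tick logic of its own in this graph.
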(event `self.ReceiveActorBeginOverlap`
  (params (OtherActor :type "Actor Object Reference"))
  (if (`self.ActorHasTag` OtherActor "Player")
    (bind _asbp_player (cast `/Game/InfiniteMatrix/Blueprints/BP_Player` OtherActor))
    (`/Game/InfiniteMatrix/Blueprints/BP_Player.ProcessHit` _asbp_player)
    (`self.K2_DestroyActor` :!label _label)
    (elif (`self.ActorHasTag` OtherActor "Projectile")
      (bind _asbp_player_2 (cast `/Game/InfiniteMatrix/Blueprints/BP_Player` (`GameplayStatics.GetPlayerPawn` 0)))
      (`/Game/InfiniteMatrix/Blueprints/BP_Player.ProcessScore` _asbp_player_2 (+ (`/Game/InfiniteMatrix/Blueprints/BP_Player.Score` _asbp_player_2) 1))
      (goto _label))))

(fn `UserConstructionScript`)